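; Per-player input receiver for the main menu character select, driving that player's golem preview, customization and ready state.
; Spawns a CH_Golem at the BP_Studio matching PlayerIndex, then registers it with the game mode.
; Inputs rotate the golem, cycle or randomize customization with deadzone and delay, and toggle Ready, which blocks customization changes.
; Select launches the game once the menu's Go image shows; ready sound pitch rises with ready player count.
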(event `InputAction|Select`
  (params (Key :type "Key Structure")))

(event `InputAction|Undo`
  (params (Key :type "Key Structure"))
  ;[1 1 1] UnReady
  (:`Pressed`
    (if (`/Game/GD/Character/Character/Golem/CH_Golem.Ready?` (`self.Spawned Player`))
      (set `/Game/GD/Character/Character/Golem/CH_Golem.Ready?` false (`self.Spawned Player`))
      (`GameplayStatics.PlaySound2D` null 0.7 1.2 0.0 null null))))

(event `InputAction|Interact/Select`
  (params (Key :type "Key Structure"))
  (bind _spawned_player (`self.Spawned Player`))
  (:`Pressed`
    (if (`Widget.IsVisible` (`/Game/GD/UI_GD/Menu/MainMenu/WBP_Lobby.Go_Image` (`self.MainMenuRef`)))
      (`/Game/GD/UI_GD/Menu/MainMenu/WBP_Lobby.LaunchGame` (`self.MainMenuRef`))
      (bind _astkt_gi (cast `/Game/GD/GameInstance/TKT_GI` (`GameplayStatics.GetGameInstance`)))
      (`/Game/GD/GameInstance/TKT_GI.StopAudio` _astkt_gi true)
      (else
        (`/Engine/EditorBlueprintResources/StandardMacros.IsValid` (`self.Spawned Player`)
          (:`Is Valid`
            (if (not (`/Game/GD/Character/Character/Golem/CH_Golem.Ready?` _spawned_player))
              (set `/Game/GD/Character/Character/Golem/CH_Golem.Ready?` true _spawned_player)
              (`GameplayStatics.PlaySound2D` (`|GetArrayItem` (`self.ReadySFXList`) (`self.PlayerIndex`)) 1.0 1.0 0.0 null null)
              (set `self.PitchToAdd` 1.0)
              (for _array_element (`/Game/GD/UI_GD/Menu/MainMenu/WBP_Lobby.CharacterSelects` (`self.MainMenuRef`))
                (if (`Widget.IsVisible` (`/Game/GD/UI_GD/Menu/MainMenu/WBP_CharacterSelect.Ready` _array_element))
                  (set `self.PitchToAdd` (+ (`self.PitchToAdd`) 0.15))))
              (`GameplayStatics.PlaySound2D` null 1.0 (`self.PitchToAdd`) 0.2 null null))))))))

(event `SpawnCharacterSelect`
  (bind _returnvalue (`GameplayStatics.GetPlayerController` (`self.PlayerIndex`)))
  (bind _spawnedplayer (`self.SpawnCharacter`))
  (bind _output_get (set `self.Spawned Player` _spawnedplayer))
  (`/Game/GD/Character/Character/Golem/CH_Golem.FirstColor` _output_get)
  (message `/Game/GD/Character/Character/Golem/BPI_GM.DisplayCharacterSelect` (`GameplayStatics.GetGameMode`) (`self.PlayerIndex`) _output_get self)
  (`/Game/Maps/MainMenu/GM_Mainmenu.AddPlayerController` (cast `/Game/Maps/MainMenu/GM_Mainmenu` (`GameplayStatics.GetGameMode`) :!pure true) _returnvalue)
  (`WidgetBlueprintLibrary.SetInputMode_GameOnly` _returnvalue)
  (set `PlayerController.bShowMouseCursor` false _returnvalue))

(event `InputAxis|Turn Right / Left Gamepad`
  (params (AxisValue :type "Float (single-precision)"))
  (`/Engine/EditorBlueprintResources/StandardMacros.IsValid` (`self.Spawned Player`)
    (:`Is Valid`
      (`self.K2_AddActorLocalRotation` (`self.Spawned Player`) (`KismetMathLibrary.MakeRotator` 0.0 0.0 (* AxisValue -3.0)) false false))))

(event `InputAxisKey|MouseX`
  (params (AxisValue :type "Float (single-precision)"))
  (`/Engine/EditorBlueprintResources/StandardMacros.IsValid` (`self.Spawned Player`)
    (:`Is Valid`
      (`self.K2_AddActorLocalRotation` (`self.Spawned Player`) (`KismetMathLibrary.MakeRotator` 0.0 0.0 (* AxisValue -2.0)) false false))))

(event `InputAxis|Move Right / Left` :consume false :overrideparent false
  (params (AxisValue :type "Float (single-precision)"))
  (bind _characterselect (`self.CharacterSelect`))
  (bind _zonemortejoystyck (`self.ZoneMorteJoystyck`))
  (if (> AxisValue 0.0)
    (if (> AxisValue _zonemortejoystyck)
      (`KismetSystemLibrary.Delay` 0.2)
      (if (not (`/Game/GD/Character/Character/Golem/CH_Golem.Ready?` (`self.Spawned Player`)))
        (`/Engine/EditorBlueprintResources/StandardMacros.IsValid` _characterselect
          (:`Is Valid`
            (`GameplayStatics.PlaySound2D` "/Game/Art/SFX/SoundEffects/UI/Change_Custom.Change_Custom" 1.0 1.5 0.0 null null)
            (`/Game/GD/Character/Character/Golem/CH_Golem.Custom` (`self.Spawned Player`) 1 (`self.CustomTypeIndex`) false)))))
    (elif (< AxisValue (* _zonemortejoystyck -1.0))
      (`KismetSystemLibrary.Delay` 0.2)
      (if (not (`/Game/GD/Character/Character/Golem/CH_Golem.Ready?` (`self.Spawned Player`)))
        (`/Engine/EditorBlueprintResources/StandardMacros.IsValid` _characterselect
          (:`Is Valid`
            (`GameplayStatics.PlaySound2D` "/Game/Art/SFX/SoundEffects/UI/Change_Custom.Change_Custom" 1.0 1.5 0.0 null null)
            (`/Game/GD/Character/Character/Golem/CH_Golem.Custom` (`self.Spawned Player`) -1 (`self.CustomTypeIndex`) false)))))))

(event `InputAxis|Move Forward / Backward` :consume false :overrideparent false
  (params (AxisValue :type "Float (single-precision)"))
  (bind _characterselect (`self.CharacterSelect`))
  (bind _zonemortejoystyck (`self.ZoneMorteJoystyck`))
  (if (> AxisValue 0.0)
    (if (> AxisValue _zonemortejoystyck)
      (`KismetSystemLibrary.Delay` 0.2)
      (if (not (`/Game/GD/Character/Character/Golem/CH_Golem.Ready?` (`self.Spawned Player`)))
        (`/Engine/EditorBlueprintResources/StandardMacros.IsValid` _characterselect
          (:`Is Valid`
            (`GameplayStatics.PlaySound2D` "/Game/Art/SFX/SoundEffects/UI/Change_Custom.Change_Custom" 1.0 1.0 0.0 null null)
            (bind _result (`/Engine/EditorBlueprintResources/StandardMacros.DecrementInt` (`self.CustomTypeIndex`))
              (:`  `
                (if (< _result 0)
                  (set `self.CustomTypeIndex` 3))))))))
    (elif (< AxisValue (* _zonemortejoystyck -1.0))
      (`KismetSystemLibrary.Delay` 0.2)
      (if (not (`/Game/GD/Character/Character/Golem/CH_Golem.Ready?` (`self.Spawned Player`)))
        (`/Engine/EditorBlueprintResources/StandardMacros.IsValid` _characterselect
          (:`Is Valid`
            (`GameplayStatics.PlaySound2D` "/Game/Art/SFX/SoundEffects/UI/Change_Custom.Change_Custom" 1.0 1.0 0.0 null null)
            (bind _result_2 (`/Engine/EditorBlueprintResources/StandardMacros.IncrementInt` (`self.CustomTypeIndex`))
              (:`  `
                (if (> _result_2 3)
                  (set `self.CustomTypeIndex` 0))))))))))

(event `InputAction|RandomizeCustom`
  (params (Key :type "Key Structure"))
  ;[1 1 1] Randomizer
  (:`Pressed`
    (if (not (`/Game/GD/Character/Character/Golem/CH_Golem.Ready?` (`self.Spawned Player`)))
      (`/Engine/EditorBlueprintResources/StandardMacros.IsValid` (`self.CharacterSelect`)
        (:`Is Valid`
          (`GameplayStatics.PlaySound2D` "/Game/Art/SFX/SoundEffects/UI/Change_Custom.Change_Custom" 1.0 1.0 0.0 null null)
          (`/Game/GD/Character/Character/Golem/CH_Golem.Custom` (`self.Spawned Player`) 0 0 true))))))

(fn `SpawnCharacter`
  (returns (SpawnedPlayer :type "/Game/GD/Character/Character/Golem/CH_Golem Object Reference"))
  (bind _outactors (`GameplayStatics.GetAllActorsOfClass` "/Game/GD/LevelElements/Studio/BP_Studio.BP_Studio_C"))
  (for _array_element _outactors
    (if (== (`/Game/GD/LevelElements/Studio/BP_Studio.SpawnIndex` _array_element) (`self.PlayerIndex`))
      (bind _returnvalue_location (`KismetMathLibrary.BreakTransform` (`self.GetTransform` _array_element)))
      (bind _returnvalue (`|SpawnActorFromClass` "/Game/GD/Character/Character/Golem/CH_Golem.CH_Golem_C" (`KismetMathLibrary.MakeTransform` _returnvalue_location (struct :`Yaw` 200.0)) "Undefined" "OverrideRootScale" null (`self.PlayerIndex`) (struct) null))
      (return _returnvalue))))

(fn `UserConstructionScript`)