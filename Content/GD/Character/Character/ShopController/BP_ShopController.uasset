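; Shop controller that lets players browse and pick bonus items for their towers in the intergame shop.
; Left/right input cycles the bonus manager's highlight and refreshes the shop UI, debounced by a short delay.
; Select only advances the game mode state; a separate ChooseBonus event adds the item's class to that player's capped tower inventory, stops the countdown timer and increments the shopped-player count.
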(event `self.ReceiveBeginPlay`
  ;[1 1 1] Comment
  (set `self.GM_Ref` (cast `/Game/Maps/Intergame/GM_InterGame` (`GameplayStatics.GetGameMode`) :!pure true)))

(event `ShopActivation`
  ;[1 1 1] Shop Activation
  (`self.ShopEnter`)
  (`KismetSystemLibrary.Delay` 0.2)
  (set `self.CanUseShopControl` true)
  (set `self.CanChooseBonus` true))

(event `ShopEnter`
  ;[1 1 1] Enter In Shop
  (`/Game/GD/LevelElements/Manager/BP_BonusManager.Highlight` (`self.BonusManagerRef`) (`self.CurrentHighlightedIndex`))
  (set `self.CurrentItemObject` (`/Game/GD/LevelElements/Manager/BP_BonusManager.LastHighlight` (`self.BonusManagerRef`)))
  (`/Game/GD/UI_GD/HUD/Shop_UI/Shop_UI.Update` (`self.ShopUIRef`)))

(event `InputAction|MenuRIght`
  (params (Key :type "Key Structure"))
  ;[1 1 1] Control In Shop
  (:`Pressed`
    (if (and (`self.CanUseShopControl`) (`self.CanChange`))
      (`GameplayStatics.PlaySound2D` "/Game/Art/SFX/SoundEffects/PickSomething/SC_MoveInmenu.SC_MoveInmenu" 1.0 1.0 0.0 null null)
      (set `self.CanChange` false)
      (bind _nextindex (`/Game/GD/LevelElements/Manager/BP_BonusManager.NextBonus` (`self.BonusManagerRef`) (`self.CurrentHighlightedIndex`)))
      (set `self.CurrentHighlightedIndex` _nextindex)
      (`/Game/GD/LevelElements/Manager/BP_BonusManager.Highlight` (`self.BonusManagerRef`) (`self.CurrentHighlightedIndex`) :!label _label)
      (set `self.CurrentItemObject` (`/Game/GD/LevelElements/Manager/BP_BonusManager.LastHighlight` (`self.BonusManagerRef`)))
      (`/Game/GD/UI_GD/HUD/Shop_UI/Shop_UI.Update` (`self.ShopUIRef`))
      (`KismetSystemLibrary.Delay` 0.15)
      (set `self.CanChange` true))))

(event `InputAction|MenuLeft`
  (params (Key :type "Key Structure"))
  ;[1 1 1] Control In Shop
  (:`Pressed`
    (if (and (`self.CanUseShopControl`) (`self.CanChange`))
      (`GameplayStatics.PlaySound2D` "/Game/Art/SFX/SoundEffects/PickSomething/SC_MoveInmenu.SC_MoveInmenu" 1.0 1.0 0.0 null null)
      (set `self.CanChange` false)
      (bind _previousindex (`/Game/GD/LevelElements/Manager/BP_BonusManager.PreviousBonus` (`self.BonusManagerRef`) (`self.CurrentHighlightedIndex`)))
      (set `self.CurrentHighlightedIndex` _previousindex)
      (goto _label))))

(event `InputAction|Interact/Select` :consume false
  (params (Key :type "Key Structure"))
  ;[1 1 1] Bonus selection
  (:`Pressed`
    (if (`self.CanChooseBonus`)
      (`/Game/Maps/Intergame/GM_InterGame.FollowingGS` (`self.GM_Ref`)))))

(event `ChooseBonus`
  (params (PlayerIndex :type Integer))
  (bind _inventory_collectables (break `/Game/GD/UI_GD/HUD/Inventory/F_Inventory` (`/Game/GD/LevelElements/Tower/CH_Tower.Inventory` (`|GetArrayItem` (`/Game/Maps/Intergame/GM_InterGame.Towers` (`self.GM_Ref`)) PlayerIndex))))
  ;[1 1 1] Bonus selection
  (bind _item_chosen (`/Game/GD/LevelElements/Manager/BP_BonusManager.ChooseItem` (`self.BonusManagerRef`) (`self.CurrentHighlightedIndex`)))
  (bind _output_get (set `self.ItemPicked` _item_chosen))
  (if (not (> (`KismetArrayLibrary.Array_Length` _inventory_collectables) 4))
    (`KismetArrayLibrary.Array_Add` _inventory_collectables (`GameplayStatics.GetObjectClass` _output_get)))
  (`KismetSystemLibrary.K2_ClearAndInvalidateTimerHandle` (`/Game/Maps/Intergame/GM_InterGame.DecreaseTimerHandler` (`self.GM_Ref`)))
  (`GameplayStatics.PlaySound2D` "/Game/Art/SFX/SoundEffects/Shop/ItemChoice.ItemChoice" 1.0 1.0 0.0 null null)
  (`/Engine/EditorBlueprintResources/StandardMacros.IncrementInt` (`/Game/Maps/Intergame/GM_InterGame.PlayerShoppedCount` (`self.GM_Ref`))
    (:`  `
      (bind _nextindex (`/Game/GD/LevelElements/Manager/BP_BonusManager.NextBonus` (`self.BonusManagerRef`) (`self.CurrentHighlightedIndex`)))
      (set `self.CurrentHighlightedIndex` _nextindex)
      (`/Game/GD/LevelElements/Manager/BP_BonusManager.Highlight` (`self.BonusManagerRef`) (`self.CurrentHighlightedIndex`))
      (set `self.CurrentItemObject` (`/Game/GD/LevelElements/Manager/BP_BonusManager.LastHighlight` (`self.BonusManagerRef`)))
      (`/Game/GD/UI_GD/HUD/Shop_UI/Shop_UI.Update` (`self.ShopUIRef`))
      (`KismetSystemLibrary.Delay` 0.15)
      (set `self.CanChange` true))))

(event `ClearShopEvent`
  ;[1 1 1] Clear shop
  (`/Game/GD/LevelElements/Manager/BP_BonusManager.ClearShop` (`self.BonusManagerRef`))
  (`/Game/GD/LevelElements/Manager/BP_BonusManager.Unhighlight` (`self.BonusManagerRef`)))

(fn `UserConstructionScript`)