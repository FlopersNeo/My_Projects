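; Cannonball projectile fired by a player in the tower level, with per-player material and Niagara trail.
; On spawn it attaches Fire or Slower effects, then moves along a fixed relative path, while a looping timer feeds travelled distance into a Material Parameter Collection for the trail.
; On impact, damage adds travel distance to any fire bonus, high values add hit VFX, and the game mode and shooter are notified to allow the next shot.
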(event `SetTrail`
  (`KismetMaterialLibrary.SetScalarParameterValue` "/Game/Art/VFX/Materials/BulletTrails/MPC_BulletTrail.MPC_BulletTrail" (`|GetArrayItem` (`self.Parameter Name`) (`self.PlayerINdex`)) (/ (`KismetMathLibrary.Vector_Distance` (`self.SpawnPoint`) (`SceneComponent.K2_GetComponentLocation` (`self.boulet`))) 1000.0)))

(event `self.ReceiveBeginPlay`
  (bind (_output_material _output_trail) (break `/Game/GD/LevelElements/Tower/F_Bullet_Mat_and_Trail` (`|GetArrayItem` (`self.F_Mat_and_Trail`) (`self.PlayerINdex`))))
  (`KismetSystemLibrary.K2_SetTimerDelegate` (delegate `SetTrail`) 0.1 true)
  (`self.SetEffect`)
  (`PrimitiveComponent.SetMaterial` (`self.boulet`) 0 _output_material)
  (`NiagaraComponent.SetAsset` (`self.Niagara`) _output_trail true)
  (set `self.SpawnPoint` (`SceneComponent.K2_GetComponentLocation` (`self.boulet`)))
  (`KismetSystemLibrary.MoveComponentTo` (`self.Scene`) (1900.0 0.0 -200.0) (struct) false false (`self.Speed`))
  (set `self.OnBackGround` true)
  (`self.destroyed`))

(event `destroyed`
  (bind _playershooter (`self.playershooter`))
  (set `self.destroyed point` (`SceneComponent.K2_GetComponentLocation` (`self.boulet`)))
  (set `self.damage` (+ (`KismetMathLibrary.Vector_Distance` (`self.SpawnPoint`) (`self.destroyed point`)) (`self.damage`)))
  (`NiagaraFunctionLibrary.SpawnSystemAtLocation` "/Game/Art/VFX/Systems/NS_CanonImpact.NS_CanonImpact" (`SceneComponent.K2_GetComponentLocation` (`self.Scene`)))
  (`/Game/Maps/Intergame/GM_InterGame.NObulletsLeft?` (cast `/Game/Maps/Intergame/GM_InterGame` (`GameplayStatics.GetGameMode`) :!pure true))
  (if (>= (`self.damage`) 1200.0)
    (`NiagaraFunctionLibrary.SpawnSystemAtLocation` "/Game/Art/VFX/Systems/NS_Hit.NS_Hit" (`SceneComponent.K2_GetComponentLocation` (`self.Scene`)))
    (set `/Game/GD/LevelElements/Tower/CH_Tower.can shoot` true _playershooter)
    (`/Game/GD/LevelElements/Tower/CH_Tower.Previsu` _playershooter)
    (if (`self.OnBackGround`)
      (`self.K2_DestroyActor`))
    (else
      (set `/Game/GD/LevelElements/Tower/CH_Tower.can shoot` true (`self.playershooter`))
      (`/Game/GD/LevelElements/Tower/CH_Tower.Previsu` (`self.playershooter`))
      (if (`self.OnBackGround`)
        (`self.K2_DestroyActor`)))))

(fn `SetEffect`
  (for (_array_element _array_index) (`self.ArrayBool`)
    (if _array_element
      (switch `name` (`|GetArrayItem` (`self.NameEffect`) _array_index)
        (:`Fire`
          (set `self.FireEffect` true)
          (set `self.damage` 200.0))
        (:`Slower`
          _))
      (`NiagaraFunctionLibrary.SpawnSystemAttached` (`|GetArrayItem` (`self.NS_Bullet`) _array_index) (`self.Niagara`) "None" (`SceneComponent.K2_GetComponentLocation` (`self.Niagara`)) (struct) "KeepWorldPosition"))))

(fn `UserConstructionScript`)