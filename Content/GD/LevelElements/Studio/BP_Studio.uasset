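; BP_Studio is a display set that presents a player's Golem with a win/lose animation, apparently for ranked results.
; SpawnSpecificPlayer spawns CH_Golem near the Scene component using the rank as player index and the player's customisation, stored as ViewingPlayer.
; Golems ranked above 1 spawn with an angled rotation.
; Rank 0 also gets Niagara confetti: one burst, then two more after a short delay.
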(event `SpawnSpecificPlayer`
  (bind (_returnvalue_location _returnvalue_rotation _returnvalue_scale) (`KismetMathLibrary.BreakTransform` (`SceneComponent.K2_GetComponentToWorld` (`self.Scene`))))
  (bind (_returnvalue_location_2 _returnvalue_rotation_2 _returnvalue_scale_2) (`KismetMathLibrary.BreakTransform` (`SceneComponent.K2_GetComponentToWorld` (`self.ConfettiSpawn`))))
  (bind (_returnvalue_location_3 _returnvalue_rotation_3 _returnvalue_scale_3) (`KismetMathLibrary.BreakTransform` (`SceneComponent.K2_GetComponentToWorld` (`self.ConfettiSpawn1`))))
  (bind (_returnvalue_location_4 _returnvalue_rotation_4 _returnvalue_scale_4) (`KismetMathLibrary.BreakTransform` (`SceneComponent.K2_GetComponentToWorld` (`self.Scene`))))
  (bind (_returnvalue_location_5 _returnvalue_rotation_5 _returnvalue_scale_5) (`KismetMathLibrary.BreakTransform` (`SceneComponent.K2_GetComponentToWorld` (`self.ConfettiSpawn2`))))
  (if (> (`self.RankNumber`) 1)
    (bind _returnvalue (`|SpawnActorFromClass` "/Game/GD/Character/Character/Golem/CH_Golem.CH_Golem_C" (`KismetMathLibrary.MakeTransform` (+ _returnvalue_location (-15.0 0.0 5.0)) (struct :`Yaw` 40.0) _returnvalue_scale) "Undefined" "OverrideRootScale" null (`self.RankNumber`) (`self.PlayerCustomisation`) null))
    (set `self.ViewingPlayer` _returnvalue)
    (else
      (bind _returnvalue_2 (`|SpawnActorFromClass` "/Game/GD/Character/Character/Golem/CH_Golem.CH_Golem_C" (`KismetMathLibrary.MakeTransform` (+ _returnvalue_location_4 (-15.0 0.0 5.0)) (struct) _returnvalue_scale_4) "Undefined" "OverrideRootScale" null (`self.RankNumber`) (`self.PlayerCustomisation`) null))
      (bind _output_get (set `self.ViewingPlayer` _returnvalue_2))))
  (`/Game/GD/Character/Character/Golem/CH_Golem.PlayWin/LoseAnim` _output_get)
  (if (== (`self.RankNumber`) 0)
    (`NiagaraFunctionLibrary.SpawnSystemAtLocation` "/Game/Art/VFX/Systems/NS_Confetti.NS_Confetti" _returnvalue_location_2 _returnvalue_rotation_2 _returnvalue_scale_2)
    (`KismetSystemLibrary.Delay` 1.5)
    (`NiagaraFunctionLibrary.SpawnSystemAtLocation` "/Game/Art/VFX/Systems/NS_Confetti.NS_Confetti" _returnvalue_location_3 _returnvalue_rotation_3 _returnvalue_scale_3)
    (`NiagaraFunctionLibrary.SpawnSystemAtLocation` "/Game/Art/VFX/Systems/NS_Confetti.NS_Confetti" _returnvalue_location_5 _returnvalue_rotation_5 _returnvalue_scale_5)))

(fn `UserConstructionScript`)