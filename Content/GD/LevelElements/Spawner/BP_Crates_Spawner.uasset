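; Spawner and referee for the floating crates minigame, where golems are eliminated by falling into the water.
; On BeginPlay it builds a grid of randomly rotated BP_Falling_Platform crates and, after a delay, starts the HUD and a one-second timer.
; The timer increases every crate's re-emerge delay at doubling intervals.
; The Laboite overlap ranks and unpossesses fallen golems, then ends the minigame when one remains.
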(event `SetWOrlMove`
  (for _array_element (`/Game/Maps/Test/GM_MinigameGolemSpawn.Players` (cast `/Game/Maps/Test/GM_MinigameGolemSpawn` (`GameplayStatics.GetGameMode`) :!pure true))
    (set `/Game/GD/Character/Character/Golem/CH_Golem.MoveOnWorldAxis?` true _array_element)))

(event `TimerEvent`
  (bind _seconds (`self.Seconds`))
  ;[1 1 1] Timer Gestion
  (`/Engine/EditorBlueprintResources/StandardMacros.IncrementInt` _seconds
    (:`  `
      (if (== _seconds 60)
        (set `self.Seconds` 0)
        (`/Engine/EditorBlueprintResources/StandardMacros.IncrementInt` (`self.Minutes`)
          (:`  `
            _)))
      (`/Engine/EditorBlueprintResources/StandardMacros.IncrementInt` (`self.UtilityCounter`)
        (:`  `
          (`self.ModifEmergeTime`))))))

(event `self.ReceiveBeginPlay`
  (bind (_returnvalue_x _returnvalue_y _returnvalue_z) (`KismetMathLibrary.BreakVector` (`self.K2_GetActorLocation`)))
  (bind _spacement (`self.Spacement`))
  ;[1 1 1] SpawnCrates
  ;;[0.1669 0 1] Timer
  (`|ExecutionSequence`
    (:`then_0`
      (`KismetSystemLibrary.Delay` 3.0)
      (bind _returnvalue (`KismetSystemLibrary.K2_SetTimerDelegate` (delegate `TimerEvent`) 1.0 true))
      (set `self.TimerObject` _returnvalue)
      (bind _returnvalue_2 (`|CreateWidget` "/Game/GD/UI_GD/HUD/Minigame/FloatingCrates/WBP_FloatingCratesHUD.WBP_FloatingCratesHUD_C" null self))
      (bind _output_get (set `self.FloatingHUDRef` _returnvalue_2))
      (`UserWidget.AddToViewport` _output_get 0))
    (:`then_1`
      (for _index (range (+ (`self.GridSize`) 1))
        (for _index_2 (range 10)
          (bind _returnvalue_3 (`|SpawnActorFromClass` "/Game/GD/LevelElements/MiniGames/BP_Falling_Platform.BP_Falling_Platform_C" (`KismetMathLibrary.MakeTransform` (`KismetMathLibrary.MakeVector` (+ _returnvalue_x (* _index_2 _spacement)) (+ _returnvalue_y (* _index _spacement)) _returnvalue_z) (`KismetMathLibrary.MakeRotator` 0.0 0.0 (`KismetArrayLibrary.Array_Random` (`self.RandomRotationList`)))) "Undefined" "OverrideRootScale" null null))
          (`KismetArrayLibrary.Array_Add` (`self.CrateList`) _returnvalue_3))))
    (:`then_2`
      (for _ (`/Game/GD/GameInstance/TKT_GI.PlayersControllerArray` (cast `/Game/GD/GameInstance/TKT_GI` (`GameplayStatics.GetGameInstance`) :!pure true))
        (`/Engine/EditorBlueprintResources/StandardMacros.IncrementInt` (`self.PlayerRank`))))))

(event `self.Laboite.OnComponentBeginOverlap`
  (params (OverlappedComponent :type "PrimitiveComponent Object Reference") (OtherActor :type "Actor Object Reference") (OtherComp :type "PrimitiveComponent Object Reference") (OtherBodyIndex :type Integer) (bFromSweep :type Boolean) (SweepResult :type "HitResult Structure (by ref)"))
  (bind _playerrank (`self.PlayerRank`))
  ;[1 1 1] Death
  (if (not (== OtherActor (`self.LastHitGolem`)))
    (bind _asch_golem (cast `/Game/GD/Character/Character/Golem/CH_Golem` OtherActor))
    (bind _output_get (set `self.LastHitGolem` _asch_golem))
    (set `/Game/GD/Character/Character/Golem/CH_Golem.MinigamePlace` _playerrank _output_get)
    (`/Engine/EditorBlueprintResources/StandardMacros.DecrementInt` _playerrank
      (:`  `
        (bind _output_get_2 (set `self.FallingLocation` (`self.K2_GetActorLocation` _output_get)))
        (`NiagaraFunctionLibrary.SpawnSystemAtLocation` "/Game/Art/VFX/Systems/NS_WaterSplash.NS_WaterSplash" _output_get_2)
        (`self.K2_SetActorLocation` (`self.LastHitGolem`) (0.0 0.0 10000.0) false true)
        (`CharacterMovementComponent.SetMovementMode` (`Character.CharacterMovement` (`self.LastHitGolem`)) "MOVE_Flying" 0)
        (`Controller.UnPossess` (`Pawn.GetController` (`self.LastHitGolem`)))
        (if (== (`self.PlayerRank`) 1)
          (bind _outactors (`GameplayStatics.GetAllActorsOfClass` "/Game/GD/Character/Character/Golem/CH_Golem.CH_Golem_C"))
          (for _array_element _outactors
            (if (== (`/Game/GD/Character/Character/Golem/CH_Golem.MinigamePlace` _array_element) 0)
              (set `/Game/GD/Character/Character/Golem/CH_Golem.MinigamePlace` 1 _array_element)
              (`/Game/GD/Character/Character/Golem/CH_Golem.ResetAnim` _array_element)
              (`Controller.UnPossess` (`Pawn.GetController` _array_element))
              (break)))
          (`Widget.RemoveFromParent` (`self.FloatingHUDRef`))
          (bind _returnvalue (`|CreateWidget` "/Game/GD/UI_GD/HUD/MinigameResult/WBP_Finish.WBP_Finish_C"))
          (`UserWidget.AddToViewport` _returnvalue 0)
          (`KismetSystemLibrary.Delay` 2.0)
          (`Widget.RemoveFromParent` _returnvalue)
          (`/Game/Maps/Test/GM_MinigameGolemSpawn.SpawnEndMinigameWidget` (cast `/Game/Maps/Test/GM_MinigameGolemSpawn` (`GameplayStatics.GetGameMode`) :!pure true)))))))

(fn `ModifEmergeTime`
  (bind _utilitycounterscale (`self.UtilityCounterScale`))
  (if (== (`self.UtilityCounter`) (`self.UtilityCounterScale`))
    (set `self.UtilityCounterScale` (+ _utilitycounterscale _utilitycounterscale))
    (for _array_element (`self.CrateList`)
      (set `/Game/GD/LevelElements/MiniGames/BP_Falling_Platform.TimeBeforeEmerge` (+ (`/Game/GD/LevelElements/MiniGames/BP_Falling_Platform.TimeBeforeEmerge` _array_element) (`self.TImeAddedBeforeEmerge`)) _array_element))
    (else
      (return))))

(fn `SpawnHUD`)

(fn `UserConstructionScript`)