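; Piranha spawner level element that keeps spawning BP_Piranha actors around its location for as long as it runs.
; On BeginPlay it starts a looping timer with a random interval picked once, and each tick has a one-in-three chance to spawn.
; Each piranha appears at a random navigable point near the spawner, so placement relies on navigation data, with random yaw and independently randomized scale on each axis.
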(event `self.ReceiveBeginPlay`
  (bind _returnvalue (`KismetSystemLibrary.K2_SetTimerDelegate` (delegate `CouldSpawnPiranha`) (`KismetMathLibrary.RandomFloatInRange` 1.0 2.0) true))
  (set `self.PiranhaSpawners` _returnvalue))

(event `CouldSpawnPiranha`
  (bind _output_get (set `self.RandomInt` (`KismetMathLibrary.RandomIntegerInRange` 0 2)))
  (if (== _output_get 0)
    (`self.SpawnPiranha`)))

(event `SpawnPiranha`
  (bind _returnvalue (`KismetMathLibrary.RandomFloatInRange` 2.0 3.0))
  (`|SpawnActorFromClass` "/Game/GD/LevelElements/Piranha/BP_Piranha.BP_Piranha_C" (`KismetMathLibrary.MakeTransform` (`NavigationSystemV1.K2_GetRandomLocationInNavigableRadius` (`self.K2_GetActorLocation`) 100.0 null null) (`KismetMathLibrary.MakeRotator` 0.0 0.0 (`KismetMathLibrary.RandomFloatInRange` 0.0 360.0)) (`KismetMathLibrary.MakeVector` _returnvalue _returnvalue _returnvalue)) "Undefined" "OverrideRootScale" null null))

(fn `UserConstructionScript`)