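; BP_Piranha is a short-lived piranha level element that plays a single jump and then removes itself.
; On BeginPlay its mesh plays the jump animation once without looping.
; After timed delays it spawns a Niagara ploof effect ahead of the mesh along the actor's forward vector, then destroys the actor.
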(event `self.ReceiveBeginPlay`
  (`SkeletalMeshComponent.PlayAnimation` (`self.Mesh`) "/Game/Art/SkeletalMeshes/SK_Piranha/A_Piraniasse_Jump.A_Piraniasse_Jump" false)
  (`KismetSystemLibrary.Delay` 0.6)
  (`NiagaraFunctionLibrary.SpawnSystemAtLocation` "/Game/Art/VFX/Systems/NS_PiranhaPloof.NS_PiranhaPloof" (+ (`SceneComponent.K2_GetComponentLocation` (`self.Mesh`)) (* (`KismetMathLibrary.GetForwardVector` (`self.K2_GetActorRotation`)) 200.0)) (struct) (0.7 0.7 0.7))
  (`KismetSystemLibrary.Delay` 0.2)
  (`self.K2_DestroyActor`))

(fn `UserConstructionScript`)