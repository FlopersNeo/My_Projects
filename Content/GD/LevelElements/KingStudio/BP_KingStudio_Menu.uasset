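; BP_KingStudio_Menu is a menu variant of the King Studio level element that spawns the menu king character when play begins.
; BeginPlay calls SpawnKing with index 0, placing CH_King_menu slightly above the Scene component with a fixed rotation and that component's scale.
; For positive indices, SpawnKing instead spawns an indexed CH_King at a fixed, distant world location and returns it, though this graph never takes that branch.
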(event `self.ReceiveBeginPlay`
  (`self.Spawn King` 0))

(fn `Spawn King`
  (params (Index :type Integer))
  (returns (ReturnValue :type "/Game/GD/LevelElements/KingStudio/CH_King Object Reference"))
  (bind (_returnvalue_location _returnvalue_rotation _returnvalue_scale) (`KismetMathLibrary.BreakTransform` (`SceneComponent.K2_GetComponentToWorld` (`self.Scene`))))
  (if (> Index 0)
    (bind _returnvalue (`|SpawnActorFromClass` "/Game/GD/LevelElements/KingStudio/CH_King.CH_King_C" (`KismetMathLibrary.MakeTransform` (1000.0 10000.0 10000.0)) "Undefined" "OverrideRootScale" null Index null))
    (return _returnvalue)
    (else
      (`|SpawnActorFromClass` "/Game/GD/LevelElements/KingStudio/CH_King_menu.CH_King_menu_C" (`KismetMathLibrary.MakeTransform` (+ _returnvalue_location (0.0 0.0 10.0)) (struct :`Pitch` 10.0 :`Yaw` -10.0) _returnvalue_scale) "Undefined" "OverrideRootScale" null 0 null)
      (return null))))

(fn `UserConstructionScript`)