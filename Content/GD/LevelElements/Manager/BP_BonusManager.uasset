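; Bonus shop manager that spawns a random collectable at each of four spawn points on BeginPlay.
; Each spawn is added to BonusList, with cube material (gold or dark matter) set by BonusListClass membership and plane materials looked up by class in CollectableMap.
; Selection uses wrap-around next/previous indices and custom-depth highlighting.
; Choosing an item removes and destroys it with a sound, while ClearShop empties the list and destroys all collectables.
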(event `SpawnBonus`
  (bind _bonuslist (`self.BonusList`))
  ;[1 1 1] Spawn
  (for _array_element (`self.SpawnerList`)
    (bind _returnvalue (`|SpawnActorFromClass` (`KismetArrayLibrary.Array_Random` (`self.CollectableList`)) (`SceneComponent.K2_GetComponentToWorld` _array_element) "Undefined" "OverrideRootScale" null null))
    (`KismetArrayLibrary.Array_Add` _bonuslist _returnvalue)
    (for _array_element_2 _bonuslist
      (if (== (`KismetArrayLibrary.Array_Find` (`self.BonusListClass`) (`GameplayStatics.GetObjectClass` _array_element_2)) -1)
        (bind _cubemesh (`/Game/GD/LevelElements/Colectables/BP_Collectables.CubeMesh` _array_element_2))
        (`PrimitiveComponent.SetMaterial` _cubemesh 0 "/Game/Art/VFX/Materials/Items/MI_DarkMatterCadre.MI_DarkMatterCadre")
        (else
          (`PrimitiveComponent.SetMaterial` _cubemesh 0 "/Game/Art/VFX/Materials/Items/MI_Gold.MI_Gold")))
      (bind _keys (`BlueprintMapLibrary.Map_Keys` (`self.CollectableMap`)))
      (for _array_element_3 _keys :!label _label
        (if (== _array_element_3 (`GameplayStatics.GetObjectClass` _array_element_2))
          (for _array_element_4 (`/Game/GD/LevelElements/Colectables/BP_Collectables.PlaneList` _returnvalue)
            (`PrimitiveComponent.SetMaterial` _array_element_4 0 (`BlueprintMapLibrary.Map_Find` (`self.CollectableMap`) _array_element_3)))
          (`self.BreakEvent`))))))

(event `BreakEvent`
  ;[1 1 1] Spawn
  (goto _label :!via `Break`))

(event `Highlight`
  (params (IndexToHighlight :type Integer))
  (bind _output (`|GetArrayItem` (`self.BonusList`) IndexToHighlight))
  (bind _cubemesh (`/Game/GD/LevelElements/Colectables/BP_Collectables.CubeMesh` _output))
  ;[1 1 1] Highlight
  (`self.Unhighlight`)
  (`/Engine/EditorBlueprintResources/StandardMacros.IsValid` _cubemesh
    (:`Is Valid`
      (`PrimitiveComponent.SetRenderCustomDepth` _cubemesh true)
      (set `self.LastHighlight` _output))))

(event `self.ReceiveBeginPlay`
  ;[1 1 1] Create list
  (set `self.SpawnerList` (`|MakeArray` (`self.SpawnPoint0`) (`self.SpawnPoint1`) (`self.SpawnPoint2`) (`self.SpawnPoint3`)))
  (`self.SpawnBonus`))

(event `Unhighlight`
  (bind _lasthighlight (`self.LastHighlight`))
  ;[1 1 1] Highlight
  (`/Engine/EditorBlueprintResources/StandardMacros.IsValid` _lasthighlight
    (:`Is Valid`
      (`PrimitiveComponent.SetRenderCustomDepth` (`/Game/GD/LevelElements/Colectables/BP_Collectables.CubeMesh` _lasthighlight) false))))

(fn `ChooseItem`
  (params (`Index to delete` :type Integer))
  (returns (`Item Chosen` :type "/Game/GD/LevelElements/Colectables/BP_Collectables Object Reference"))
  (locals (Result :type "/Game/GD/LevelElements/Colectables/BP_Collectables Object Reference"))
  (bind _bonuslist (`self.BonusList`))
  (set `local.Result` (`|GetArrayItem` _bonuslist `Index to delete`))
  (`KismetArrayLibrary.Array_Remove` _bonuslist `Index to delete`)
  (`self.K2_DestroyActor` (`local.Result`))
  (`GameplayStatics.PlaySound2D` null 1.0 1.0 0.0 null null)
  (return (`local.Result`)))

(fn `ClearShop`
  (`KismetArrayLibrary.Array_Clear` (`self.BonusList`))
  (bind _outactors (`GameplayStatics.GetAllActorsOfClass` "/Game/GD/LevelElements/Colectables/BP_Collectables.BP_Collectables_C"))
  (`self.K2_DestroyActor` _outactors))

(fn `NextBonus`
  (params (CurentIndex :type Integer))
  (returns (NextIndex :type Integer))
  (locals (TempIndex :type Integer))
  (bind _output_get (set `local.TempIndex` (+ CurentIndex 1)))
  (if (not (`KismetArrayLibrary.Array_IsValidIndex` (`self.BonusList`) _output_get))
    (set `local.TempIndex` 0))
  (return (`local.TempIndex`)))

(fn `PreviousBonus`
  (params (CurrentIndex :type Integer))
  (returns (PreviousIndex :type Integer))
  (locals (TempIndex :type Integer))
  (bind _output_get (set `local.TempIndex` (- CurrentIndex 1)))
  (if (not (`KismetArrayLibrary.Array_IsValidIndex` (`self.BonusList`) _output_get))
    (set `local.TempIndex` (`KismetArrayLibrary.Array_LastIndex` (`self.BonusList`))))
  (return (`local.TempIndex`)))

(fn `UserConstructionScript`)