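; BP_Coconut is a falling coconut projectile for a minigame that damages golems it touches.
; On BeginPlay, a latent MoveComponentTo lowers its sphere with random rotation over CoconutSpeed, then destroys the actor.
; Overlapping a CH_Golem applies damage using the game mode's Rank; other non-coconut overlaps spawn an impact Niagara effect, and both destroy it.
; A separate Hit event also destroys the coconut.
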(event `self.ReceiveHit`
  (params (MyComp :type "PrimitiveComponent Object Reference") (Other :type "Actor Object Reference") (OtherComp :type "PrimitiveComponent Object Reference") (bSelfMoved :type Boolean) (HitLocation :type "Vector Structure") (HitNormal :type "Vector Structure") (NormalImpulse :type "Vector Structure") (Hit :type "HitResult Structure (by ref)"))
  ;[1 1 1] Hit event
  (`self.K2_DestroyActor`))

(event `self.ReceiveBeginPlay`
  ;[1 1 1] BeginPlay
  (`KismetSystemLibrary.MoveComponentTo` (`self.Sphere`) (0.0 0.0 -800.0) (`KismetMathLibrary.MakeRotator` (`KismetMathLibrary.RandomFloatInRange` -180.0 180.0) (`KismetMathLibrary.RandomFloatInRange` -180.0 180.0) (`KismetMathLibrary.RandomFloatInRange` -180.0 180.0)) false false (`self.CoconutSpeed`))
  (`self.K2_DestroyActor`))

(event `self.Damage.OnComponentBeginOverlap`
  (params (OverlappedComponent :type "PrimitiveComponent Object Reference") (OtherActor :type "Actor Object Reference") (OtherComp :type "PrimitiveComponent Object Reference") (OtherBodyIndex :type Integer) (bFromSweep :type Boolean) (SweepResult :type "HitResult Structure (by ref)"))
  ;[1 1 1] SpawnVFX
  (bind _asch_golem (cast `/Game/GD/Character/Character/Golem/CH_Golem` OtherActor)
    (:`then`
      (`/Game/GD/Character/Character/Golem/CH_Golem.Damaged` _asch_golem (`/Game/Maps/Test/GM_MinigameGolemSpawn.Rank` (cast `/Game/Maps/Test/GM_MinigameGolemSpawn` (`GameplayStatics.GetGameMode`) :!pure true))))
    (:`CastFailed`
      (cast `/Game/GD/LevelElements/MiniGames/Coconut/BP_Coconut` OtherActor
        (:`CastFailed`
          (`NiagaraFunctionLibrary.SpawnSystemAtLocation` "/Game/Art/VFX/Systems/NS_CoconutImpact.NS_CoconutImpact" (`SceneComponent.K2_GetComponentLocation` (`self.Sphere`)) (struct) (0.7 0.7 0.7))))))
  (`self.K2_DestroyActor`))

(fn `UserConstructionScript`)