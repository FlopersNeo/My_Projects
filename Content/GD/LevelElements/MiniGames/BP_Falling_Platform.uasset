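; Floating crate platform for minigames that sinks under a possessed CH_Golem and later resurfaces.
; Trigger overlap starts short delays, then sinks the crate if it can move and the golem is possessed.
; Sinks plays the sinking animation and disables RealCollision, waits TimeBeforeEmerge, then plays the rising animation before restoring collision.
; CanMove blocks new sinks during the cycle, though it is checked before the last delay.
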(event `self.ReceiveBeginPlay`
  ;[1 1 1] Anim
  (`SkeletalMeshComponent.PlayAnimation` (`self.SkeletalMesh`) "/Game/Art/SkeletalMeshes/SK_Crate/SK_Crate_Anim_Box_Armature_Armature_Crate_Floating_Armature_Crate_Floating.SK_Crate_Anim_Box_Armature_Armature_Crate_Floating_Armature_Crate_Floating" true))

(event `self.Trigger.OnComponentBeginOverlap`
  (params (OverlappedComponent :type "PrimitiveComponent Object Reference") (OtherActor :type "Actor Object Reference") (OtherComp :type "PrimitiveComponent Object Reference") (OtherBodyIndex :type Integer) (bFromSweep :type Boolean) (SweepResult :type "HitResult Structure (by ref)"))
  ;[1 1 1] Comment
  (bind _asch_golem (cast `/Game/GD/Character/Character/Golem/CH_Golem` OtherActor))
  (if (not (`/Game/GD/Character/Character/Golem/CH_Golem.Possessed` _asch_golem))
    (`KismetSystemLibrary.Delay` 0.5))
  (if (`self.CanMove?`)
    (`KismetSystemLibrary.Delay` 0.5)
    (if (`/Game/GD/Character/Character/Golem/CH_Golem.Possessed` _asch_golem)
      (`self.Sinks`))))

(event `Sinks`
  ;[1 1 1] Crates Movement
  ;;[0.7776 0 1] Sinking
  (`SkeletalMeshComponent.PlayAnimation` (`self.SkeletalMesh`) "/Game/Art/SkeletalMeshes/SK_Crate/SK_Crate_Anim_Box_Armature_Armature_Crate_Sinking_Armature_Crate_Sinking.SK_Crate_Anim_Box_Armature_Armature_Crate_Sinking_Armature_Crate_Sinking" false)
  (`PrimitiveComponent.SetCollisionEnabled` (`self.RealCollision`) "NoCollision")
  (set `self.CanMove?` false)
  ;;[0 1 0.1674] Drowned
  (`KismetSystemLibrary.Delay` (`self.TimeBeforeEmerge`))
  ;;[1 0.7328 0] Emerge
  (`SkeletalMeshComponent.PlayAnimation` (`self.SkeletalMesh`) "/Game/Art/SkeletalMeshes/SK_Crate/SK_Crate_Anim_Box_Armature_Armature_Crate_GoingUp_Armature_Crate_GoingUp.SK_Crate_Anim_Box_Armature_Armature_Crate_GoingUp_Armature_Crate_GoingUp" false)
  (`KismetSystemLibrary.Delay` 1.65)
  (`PrimitiveComponent.SetCollisionEnabled` (`self.RealCollision`) "QueryAndPhysics")
  (set `self.CanMove?` true))

(fn `UserConstructionScript`)