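; Game mode for the endgame map that stages a suspenseful, spotlit reveal of players ranked by their damage.
; BeginPlay sorts player indices from the game instance's damage totals, then spawns each customised golem at a PlayerStart in that order.
; Suspense identifies three spotlights by cone angle, blacks them out, lights the middle one with sound cues, then possesses the golems.
; A timeline then animates all three lights and post-process exposure.
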(event `Suspense`
  (`GameplayStatics.PlaySound2D` "/Game/Art/SFX/SoundEffects/Suspense.Suspense" 1.0 1.0 0.0 null null)
  (bind _returnvalue (`GameplayStatics.GetActorOfClass` "/Script/Engine.PostProcessVolume"))
  (bind _output_get (set `self.PostProcessVolume` _returnvalue))
  (set `PostProcessVolume.Settings` (make `PostProcessSettings` :`AutoExposureMethod` "AEM_Manual" :`ColorContrast` (1.14 1.14 1.14 1.0) :`AutoExposureBias` 5.0 :`VignetteIntensity` 0.416) _output_get)
  (bind _outactors (`GameplayStatics.GetAllActorsOfClass` "/Script/Engine.SpotLight"))
  (for _array_element _outactors
    (bind _spotlightcomponent (`SpotLight.SpotLightComponent` _array_element))
    (if (== (`SpotLightComponent.OuterConeAngle` _spotlightcomponent) 27.0)
      (set `self.MidSpotLight` _array_element)
      (elif (== (`SpotLightComponent.OuterConeAngle` _spotlightcomponent) 44.0)
        (set `self.LeftSpot` _array_element)
        (else
          (set `self.RightSpot` _array_element)))))
  (`LightComponent.SetIntensity` (`Light.LightComponent` (`self.LeftSpot`)) 0.0)
  (`LightComponent.SetIntensity` (`Light.LightComponent` (`self.RightSpot`)) 0.0)
  (`LightComponent.SetIntensity` (`Light.LightComponent` (`self.MidSpotLight`)) 0.0)
  (`KismetSystemLibrary.Delay` 4.2)
  (`GameplayStatics.PlaySound2D` "/Game/Art/SFX/SoundEffects/Endgame/SpotLightOn.SpotLightOn" 1.0 1.0 0.0 null null)
  (`LightComponent.SetIntensity` (`Light.LightComponent` (`self.MidSpotLight`)) 1500.0)
  (`KismetSystemLibrary.Delay` 2.0)
  (for (_array_element_2 _array_index) (`self.Players`)
    (`Controller.Possess` (`GameplayStatics.GetPlayerController` (`|GetArrayItem` (`self.Players IndexSORTED`) _array_index)) _array_element_2))
  (bind (_direction _leftlight _rightlight _exposure _mdilight) (`Timeline|Timeline_0` :!via `PlayFromStart`)
    (:`Update`
      (`LightComponent.SetIntensity` (`SpotLight.SpotLightComponent` (`self.LeftSpot`)) _leftlight)
      (`LightComponent.SetIntensity` (`SpotLight.SpotLightComponent` (`self.RightSpot`)) _rightlight)
      (set `PostProcessVolume.Settings` (make `PostProcessSettings` :`AutoExposureMethod` "AEM_Manual" :`ColorContrast` (1.14 1.14 1.14 1.0) :`AutoExposureBias` _exposure :`VignetteIntensity` 0.416) (`self.PostProcessVolume`))
      (`LightComponent.SetIntensity` (`SpotLight.SpotLightComponent` (`self.MidSpotLight`)) _mdilight))))

(event `self.ReceiveBeginPlay`
  (`/Game/GD/GameInstance/TKT_GI.StopAudio` (cast `/Game/GD/GameInstance/TKT_GI` (`GameplayStatics.GetGameInstance`) :!pure true) false)
  (bind _outactors (`GameplayStatics.GetAllActorsOfClass` "/Script/Engine.PlayerStart"))
  (set `self.PlayerStartArray` _outactors)
  (bind _playersindex (`self.SortPlayers`))
  (set `self.Players IndexSORTED` _playersindex)
  (for (_ _array_index) (`/Game/GD/GameInstance/TKT_GI.PlayersControllerArray` (cast `/Game/GD/GameInstance/TKT_GI` (`GameplayStatics.GetGameInstance`) :!pure true))
    (`self.SpawnPlayer` (`|GetArrayItem` (`self.Players IndexSORTED`) _array_index) (`|GetArrayItem` (`self.PlayerStartArray`) _array_index)))
  (`self.Suspense`))

(fn `DisplayCharacterSelect`
  (params (CurrentPlayerIndex :type Integer) (Player :type "/Game/GD/Character/Character/Golem/CH_Golem Object Reference") (InputReceiver :type "/Game/GD/Character/Character/Golem/BP_InputReceiver Object Reference"))
  (returns (Return :type Boolean))
  (return false))

(fn `MenuSpawnPlayer`
  (params (CurrentPlayerIndex :type Integer) (PlayerStart :type "/Game/GD/LevelElements/Studio/BP_Studio Object Reference"))
  (returns (Return :type Boolean))
  (return false))

(fn `SaveCustomisationToGameInstance`
  (returns (Return :type Boolean))
  (return false))

(fn `SortPlayers`
  (returns (PlayersIndex :type "Array of Integer"))
  (locals (GameInstance :type "/Game/GD/GameInstance/TKT_GI Object Reference") (SortedPlayerIndex :type "Array of Integer") (PlayerDamageCopy :type "Array of Integer"))
  (bind _gameinstance (`local.GameInstance`))
  (bind _astkt_gi (cast `/Game/GD/GameInstance/TKT_GI` (`GameplayStatics.GetGameInstance`) :!pure true))
  (set `local.GameInstance` _astkt_gi)
  (bind _output_get (set `local.PlayerDamageCopy` (`/Game/GD/GameInstance/TKT_GI.PlayersDamage` _astkt_gi)))
  (for (_array_element _array_index) _output_get
    (for (_array_element_2 _array_index_2) (`local.PlayerDamageCopy`)
      (if (> _array_element _array_element_2)
        (`KismetArrayLibrary.Array_Swap` (`local.PlayerDamageCopy`) _array_index _array_index_2))))
  (for (_ _array_index_3) (`/Game/GD/GameInstance/TKT_GI.PlayersControllerArray` _gameinstance)
    (for (_array_element_3 _array_index_4) (`/Game/GD/GameInstance/TKT_GI.PlayersDamage` _gameinstance)
      (if (== _array_element_3 (`|GetArrayItem` (`local.PlayerDamageCopy`) _array_index_3))
        (`KismetArrayLibrary.Array_Add` (`local.SortedPlayerIndex`) _array_index_4))))
  (return (`local.SortedPlayerIndex`)))

(fn `SpawnPlayer`
  (params (CurrentPlayerIndex :type Integer) (PlayerStart :type "PlayerStart Object Reference"))
  (returns (Return :type Boolean))
  (bind _currentplayerindex (`local.CurrentPlayerIndex`))
  (`/Engine/EditorBlueprintResources/StandardMacros.IsValid` (`GameplayStatics.GetPlayerController` (`local.CurrentPlayerIndex`))
    (:`Is Valid`
      (bind _returnvalue (`|SpawnActorFromClass` "/Game/GD/Character/Character/Golem/CH_Golem.CH_Golem_C" (`self.GetTransform` PlayerStart) "Undefined" "OverrideRootScale" null _currentplayerindex (`|GetArrayItem` (`/Game/GD/GameInstance/TKT_GI.PlayersCustomisationArray` (cast `/Game/GD/GameInstance/TKT_GI` (`GameplayStatics.GetGameInstance`) :!pure true)) _currentplayerindex) null))
      (`KismetArrayLibrary.Array_Add` (`self.Players`) _returnvalue)
      (set `/Game/GD/Character/Character/Golem/CH_Golem.MoveOnWorldAxis?` true _returnvalue)
      (return false))))

(fn `UserConstructionScript`)