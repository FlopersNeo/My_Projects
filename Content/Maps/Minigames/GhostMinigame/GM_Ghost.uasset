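; Game mode for the Ghost minigame that spawns and possesses a customised CH_Golem at a PlayerStart for each player.
; No gameplay runs here: EndMinigame follows a short Delay after spawning and assigns unique random places through recursive re-rolls, saving them to the game instance.
; It then spawns a BP_Studio per player in rank order, routes each camera to that player's render target, and shows WBP_MinigameResult.
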(event `self.ReceiveBeginPlay`
  (bind _outactors (`GameplayStatics.GetAllActorsOfClass` "/Script/Engine.PlayerStart"))
  (for (_ _array_index) (`/Game/GD/GameInstance/TKT_GI.PlayersControllerArray` (cast `/Game/GD/GameInstance/TKT_GI` (`GameplayStatics.GetGameInstance`) :!pure true))
    (`self.SpawnPlayer` _array_index (`|GetArrayItem` _outactors _array_index))
    (`KismetSystemLibrary.Delay` 1.0)
    (`self.EndMinigame`)))

(fn `DisplayCharacterSelect`
  (params (CurrentPlayerIndex :type Integer) (Player :type "/Game/GD/Character/Character/Golem/CH_Golem Object Reference") (InputReceiver :type "/Game/GD/Character/Character/Golem/BP_InputReceiver Object Reference"))
  (returns (Return :type Boolean))
  (return false))

(fn `EndMinigame`
  (bind _playerslastminigameplace (`/Game/GD/GameInstance/TKT_GI.PlayersLastMinigamePlace` (cast `/Game/GD/GameInstance/TKT_GI` (`GameplayStatics.GetGameInstance`) :!pure true)))
  (`KismetArrayLibrary.Array_Clear` _playerslastminigameplace)
  (for _array_element (`self.Players`)
    (bind _index (`self.GetRandomPlace`))
    (bind _output_get (set `/Game/GD/Character/Character/Golem/CH_Golem.MinigamePlace` _index _array_element))
    (`KismetArrayLibrary.Array_Add` _playerslastminigameplace _output_get))
  (for _ (`self.Players`)
    (bind _result (`/Engine/EditorBlueprintResources/StandardMacros.IncrementInt` (`self.SortPlayerIndex`))
      (:`  `
        (for (_array_element_2 _array_index) (`/Game/GD/GameInstance/TKT_GI.PlayersLastMinigamePlace` (cast `/Game/GD/GameInstance/TKT_GI` (`GameplayStatics.GetGameInstance`) :!pure true))
          (if (== _array_element_2 _result)
            (set `self.PlayerIndex` _array_index)
            (bind _returnvalue (`|SpawnActorFromClass` "/Game/GD/LevelElements/Studio/BP_Studio.BP_Studio_C" (`|GetArrayItem` (`self.StudioSpawn`) _array_index) "Undefined" "OverrideRootScale" null _array_index (`/Game/GD/Character/Character/Golem/CH_Golem.Customisation` (`|GetArrayItem` (`self.Players`) _array_index)) (- (`self.SortPlayerIndex`) 1) null))
            (`KismetArrayLibrary.Array_Add` (`self.Studios`) _returnvalue)
            (`/Game/GD/LevelElements/Studio/BP_Studio.SpawnSpecificPlayer` _returnvalue)
            (switch `int` (`self.PlayerIndex`)
              (:`0`
                (bind _cam (`/Game/GD/LevelElements/Studio/BP_Studio.cam` _returnvalue))
                (set `SceneCaptureComponent2D.TextureTarget` "/Game/GD/LevelElements/Studio/RT_P1.RT_P1" _cam))
              (:`1`
                (set `SceneCaptureComponent2D.TextureTarget` "/Game/GD/LevelElements/Studio/RT_P2.RT_P2" _cam))
              (:`2`
                (set `SceneCaptureComponent2D.TextureTarget` "/Game/GD/LevelElements/Studio/RT_P3.RT_P3" _cam))
              (:`3`
                (set `SceneCaptureComponent2D.TextureTarget` "/Game/GD/LevelElements/Studio/RT_P4.RT_P4" _cam))))))))
  (bind _returnvalue_2 (`|CreateWidget` "/Game/GD/UI_GD/HUD/MinigameResult/WBP_MinigameResult.WBP_MinigameResult_C" null (`self.Studios`) (`/Game/GD/GameInstance/TKT_GI.PlayersCustomisationArray` (cast `/Game/GD/GameInstance/TKT_GI` (`GameplayStatics.GetGameInstance`) :!pure true))))
  (`UserWidget.AddToViewport` _returnvalue_2 0))

(fn `GetRandomPlace`
  (returns (Index :type Integer))
  (bind _output_get (set `self.Index` (`KismetMathLibrary.RandomIntegerInRange` 1 (`KismetArrayLibrary.Array_Length` (`self.Players`)))))
  (if (`KismetArrayLibrary.Array_Contains` (`self.Place`) _output_get)
    (`self.GetRandomPlace`)
    (else
      (`KismetArrayLibrary.Array_Add` (`self.Place`) _output_get)
      (return _output_get))))

(fn `MenuSpawnPlayer`
  (params (CurrentPlayerIndex :type Integer) (PlayerStart :type "/Game/GD/LevelElements/Studio/BP_Studio Object Reference"))
  (returns (Return :type Boolean))
  (return false))

(fn `SaveCustomisationToGameInstance`
  (returns (Return :type Boolean))
  (return false))

(fn `SpawnPlayer`
  (params (CurrentPlayerIndex :type Integer) (PlayerStart :type "PlayerStart Object Reference"))
  (returns (Return :type Boolean))
  (bind _currentplayerindex (`local.CurrentPlayerIndex`))
  (`/Engine/EditorBlueprintResources/StandardMacros.IsValid` (`GameplayStatics.GetPlayerController` (`local.CurrentPlayerIndex`))
    (:`Is Valid`
      (bind _returnvalue (`|SpawnActorFromClass` "/Game/GD/Character/Character/Golem/CH_Golem.CH_Golem_C" (`self.GetTransform` PlayerStart) "Undefined" "OverrideRootScale" null _currentplayerindex (`|GetArrayItem` (`/Game/GD/GameInstance/TKT_GI.PlayersCustomisationArray` (cast `/Game/GD/GameInstance/TKT_GI` (`GameplayStatics.GetGameInstance`) :!pure true)) _currentplayerindex) null))
      (`Controller.Possess` (`GameplayStatics.GetPlayerController` (`local.CurrentPlayerIndex`)) _returnvalue)
      (`KismetArrayLibrary.Array_Add` (`self.Players`) _returnvalue)
      (return false))))

(fn `UserConstructionScript`)