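; BP_CoconutTimer is the elapsed-time counter for the coconut minigame and also spawns that minigame's health HUD.
; On BeginPlay, a looping one-second timer increments Seconds and rolls it over into Minutes.
; After a short delay, it adds WBP_CocoNutHealth to the viewport, passing itself and the Players from GM_MinigameGolemSpawn.
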(event `TimerConnard`
  (bind _seconds (`self.Seconds`))
  (`/Engine/EditorBlueprintResources/StandardMacros.IncrementInt` _seconds
    (:`  `
      (if (== _seconds 60)
        (set `self.Seconds` 0)
        (`/Engine/EditorBlueprintResources/StandardMacros.IncrementInt` (`self.Minutes`))))))

(event `self.ReceiveBeginPlay`
  (`KismetSystemLibrary.K2_SetTimerDelegate` (delegate `TimerConnard`) 1.0 true)
  (`KismetSystemLibrary.Delay` 3.0)
  (bind _returnvalue (`|CreateWidget` "/Game/Maps/Minigames/Coconut_Minigame/WBP_CocoNutHealth.WBP_CocoNutHealth_C" null self (`/Game/Maps/Test/GM_MinigameGolemSpawn.Players` (cast `/Game/Maps/Test/GM_MinigameGolemSpawn` (`GameplayStatics.GetGameMode`) :!pure true))))
  (`UserWidget.AddToViewport` _returnvalue 0))

(fn `UserConstructionScript`)