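; Minigame game mode that spawns a customised CH_Golem per player controller stored in the game instance and runs the match intro and results.
; BeginPlay drives a rail camera by timeline, shows a start widget, then possesses the golems and hides their info.
; SpawnEndMinigameWidget saves placings, spawns ranked BP_Studio captures into per-player render targets for the result widget, and stops audio.
; Several menu and customisation functions are empty stubs.
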(event `self.ReceiveBeginPlay`
  (`|ExecutionSequence`
    (:`then_0`
      (`self.GetPlayerStartPoints`)
      (for (_ _array_index) (`/Game/GD/GameInstance/TKT_GI.PlayersControllerArray` (cast `/Game/GD/GameInstance/TKT_GI` (`GameplayStatics.GetGameInstance`) :!pure true))
        (`/Game/GD/Character/Character/Golem/BPI_GM.SpawnPlayer` _array_index (`|GetArrayItem` (`self.PlayerStartArray`) _array_index))))
    (:`then_1`
      (for _array_element (`self.Players`)
        (`/Game/GD/Character/Character/Golem/CH_Golem.SetPlayerInfoVisble` _array_element)
        (set `/Game/GD/Character/Character/Golem/CH_Golem.Possessed` true _array_element))
      (bind _outactors (`GameplayStatics.GetAllActorsOfClass` "/Script/CinematicCamera.CameraRig_Rail"))
      (bind (_direction _newtrack_0) (`Timeline|Timeline_0` :!via `PlayFromStart`)
        (:`Update`
          (set `CameraRig_Rail.CurrentPositionOnRail` _newtrack_0 (`|GetArrayItem` _outactors)))
        (:`Finished`
          (bind _returnvalue (`|CreateWidget` "/Game/GD/UI_GD/HUD/MinigameResult/WBP_Start.WBP_Start_C"))
          (`UserWidget.AddToViewport` _returnvalue 0)
          (`KismetSystemLibrary.Delay` 1.7)
          (`Widget.RemoveFromParent` _returnvalue)
          (for (_array_element_2 _array_index_2) (`self.Players`)
            (`Controller.Possess` (`GameplayStatics.GetPlayerController` _array_index_2) _array_element_2))
          (`KismetSystemLibrary.Delay` 1.0)
          (for _array_element_3 (`self.Players`)
            (`/Game/GD/Character/Character/Golem/CH_Golem.SetPlayerInfoHidden` _array_element_3)))))
    (:`then_2`
      (for _ (`self.Players`)
        (`/Engine/EditorBlueprintResources/StandardMacros.IncrementInt` (`self.Rank`))))))

(event `SpawnEndMinigameWidget`
  (bind _playerslastminigameplace (`/Game/GD/GameInstance/TKT_GI.PlayersLastMinigamePlace` (cast `/Game/GD/GameInstance/TKT_GI` (`GameplayStatics.GetGameInstance`) :!pure true)))
  (`KismetArrayLibrary.Array_Clear` _playerslastminigameplace)
  (for _array_element (`self.Players`)
    (`KismetArrayLibrary.Array_Add` _playerslastminigameplace (`/Game/GD/Character/Character/Golem/CH_Golem.MinigamePlace` _array_element)))
  (for _ (`self.Players`)
    (bind _result (`/Engine/EditorBlueprintResources/StandardMacros.IncrementInt` (`self.SortPlayerIndex`))
      (:`  `
        (for (_array_element_2 _array_index) (`/Game/GD/GameInstance/TKT_GI.PlayersLastMinigamePlace` (cast `/Game/GD/GameInstance/TKT_GI` (`GameplayStatics.GetGameInstance`) :!pure true))
          (if (== _array_element_2 _result)
            (set `self.PlayerIndex` _array_index)
            (bind _returnvalue (`|SpawnActorFromClass` "/Game/GD/LevelElements/Studio/BP_Studio.BP_Studio_C" (`|GetArrayItem` (`self.StudioSpawn`) _array_index) "Undefined" "OverrideRootScale" null _array_index (`/Game/GD/Character/Character/Golem/CH_Golem.Customisation` (`|GetArrayItem` (`self.Players`) _array_index)) (- (`self.SortPlayerIndex`) 1) null))
            (`KismetArrayLibrary.Array_Add` (`self.Studios`) _returnvalue)
            (`/Game/GD/LevelElements/Studio/BP_Studio.SpawnSpecificPlayer` _returnvalue)
            (switch `int` (`self.PlayerIndex`)
              (:`0`
                (bind _cam (`/Game/GD/LevelElements/Studio/BP_Studio.cam` _returnvalue))
                (set `SceneCaptureComponent2D.TextureTarget` "/Game/GD/LevelElements/Studio/RT_P1.RT_P1" _cam))
              (:`1`
                (set `SceneCaptureComponent2D.TextureTarget` "/Game/GD/LevelElements/Studio/RT_P2.RT_P2" _cam))
              (:`2`
                (set `SceneCaptureComponent2D.TextureTarget` "/Game/GD/LevelElements/Studio/RT_P3.RT_P3" _cam))
              (:`3`
                (set `SceneCaptureComponent2D.TextureTarget` "/Game/GD/LevelElements/Studio/RT_P4.RT_P4" _cam))))))))
  (bind _returnvalue_2 (`|CreateWidget` "/Game/GD/UI_GD/HUD/MinigameResult/WBP_MinigameResult.WBP_MinigameResult_C" null (`self.Studios`) (`/Game/GD/GameInstance/TKT_GI.PlayersCustomisationArray` (cast `/Game/GD/GameInstance/TKT_GI` (`GameplayStatics.GetGameInstance`) :!pure true))))
  (`UserWidget.AddToViewport` _returnvalue_2 0)
  (bind _astkt_gi (cast `/Game/GD/GameInstance/TKT_GI` (`GameplayStatics.GetGameInstance`)))
  (`/Game/GD/GameInstance/TKT_GI.StopAudio` _astkt_gi true))

(fn `DisplayCharacterSelect`
  (params (CurrentPlayerIndex :type Integer) (Player :type "/Game/GD/Character/Character/Golem/CH_Golem Object Reference") (InputReceiver :type "/Game/GD/Character/Character/Golem/BP_InputReceiver Object Reference"))
  (returns (Return :type Boolean))
  (return false))

(fn `GetPlayerStartPoints`
  (bind _outactors (`GameplayStatics.GetAllActorsOfClass` "/Script/Engine.PlayerStart"))
  (set `self.PlayerStartArray` _outactors))

(fn `MenuSpawnPlayer`
  (params (CurrentPlayerIndex :type Integer) (PlayerStart :type "/Game/GD/LevelElements/Studio/BP_Studio Object Reference"))
  (returns (Return :type Boolean))
  (return false))

(fn `NameToInt`
  (params (PlayerStart :type "PlayerStart Object Reference"))
  (returns (ReturnValue :type Integer))
  (return (`KismetStringLibrary.Conv_StringToInt` (`KismetStringLibrary.Conv_NameToString` (`PlayerStart.PlayerStartTag` PlayerStart)))))

(fn `SaveCustomisationToGameInstance`
  (returns (Return :type Boolean))
  (return false))

(fn `SpawnInputReceivers`
  (locals (Index :type Integer))
  (bind _returnvalue (`GameplayStatics.GetPlayerController` (`local.Index`)))
  (for (_ _array_index) (`self.PlayerStartArray`)
    (set `local.Index` _array_index)
    (for _array_element (`self.PlayerStartArray`)
      (if (== (`self.NameToInt` _array_element) (`local.Index`))
        (`GameplayStatics.CreatePlayer` -1)
        (bind _returnvalue_2 (`|SpawnActorFromClass` "/Game/GD/Character/Character/Golem/BP_InputReceiver.BP_InputReceiver_C" (`self.GetTransform` (`|GetArrayItem` (`self.PlayerStartArray`) (`local.Index`))) "Undefined" "OverrideRootScale" null (`local.Index`) null null null))
        (`KismetArrayLibrary.Array_AddUnique` (`self.PlayerInputReceiverArray`) _returnvalue_2)
        (`Controller.Possess` _returnvalue _returnvalue_2)
        (`KismetArrayLibrary.Array_AddUnique` (`self.PlayerControllerArray`) _returnvalue)))))

(fn `SpawnPlayer`
  (params (CurrentPlayerIndex :type Integer) (PlayerStart :type "PlayerStart Object Reference"))
  (returns (Return :type Boolean))
  (bind _currentplayerindex (`local.CurrentPlayerIndex`))
  (`/Engine/EditorBlueprintResources/StandardMacros.IsValid` (`GameplayStatics.GetPlayerController` (`local.CurrentPlayerIndex`))
    (:`Is Valid`
      (bind _returnvalue (`|SpawnActorFromClass` "/Game/GD/Character/Character/Golem/CH_Golem.CH_Golem_C" (`self.GetTransform` PlayerStart) "Undefined" "OverrideRootScale" null _currentplayerindex (`|GetArrayItem` (`/Game/GD/GameInstance/TKT_GI.PlayersCustomisationArray` (cast `/Game/GD/GameInstance/TKT_GI` (`GameplayStatics.GetGameInstance`) :!pure true)) _currentplayerindex) null))
      (`KismetArrayLibrary.Array_Add` (`self.Players`) _returnvalue)
      (return false))))

(fn `UserConstructionScript`)